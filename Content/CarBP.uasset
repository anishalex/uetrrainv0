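; CarBP is a drivable vehicle Blueprint with a mouse-controlled spring arm camera.
; Steering, throttle, brake and handbrake inputs pass straight to the VehicleMovementComponent.
; Mouse X and Y add yaw and pitch rotation to the SpringArm.
; Tick draws a debug sphere at the mesh's center of mass to visualize it while driving.
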(event EventBeginPlay)

(event Collision|EventActorBeginOverlap
  (params (OtherActor :type Actor%20Object%20Reference)))

(event EventTick
  (params (DeltaSeconds :type Float%20%28single-precision%29))
  (Rendering|Debug|DrawDebugSphere (Physics|GetCenterOfMass (Variables|Character|GetMesh) "None") 1e+02 12 "(R=1.000000,G=0.085571,B=0.369045,A=1.000000)" 0.0))

(event Input|ActionEvents|InputActionhandbrake
  (params (Key :type Key%20Structure :default "None"))
  (bind _vehiclemovementcomponent (Variables|Default|GetVehicleMovementComponent))
  ;[1 1 1] axis and actions
  (:Pressed
    (Class|ChaosVehicleMovementComponent|SetHandbrakeInput _vehiclemovementcomponent true))
  (:Released
    (Class|ChaosVehicleMovementComponent|SetHandbrakeInput _vehiclemovementcomponent false)))

(event Input|AxisEvents|InputAxisbrake
  (params (AxisValue :type Float%20%28single-precision%29))
  ;[1 1 1] axis and actions
  (Class|ChaosVehicleMovementComponent|SetBrakeInput (Variables|Default|GetVehicleMovementComponent) AxisValue))

(event Input|AxisEvents|InputAxissteering
  (params (AxisValue :type Float%20%28single-precision%29))
  ;[1 1 1] axis and actions
  (Class|ChaosVehicleMovementComponent|SetSteeringInput (Variables|Default|GetVehicleMovementComponent) AxisValue))

(event Input|AxisEvents|InputAxisthrottle
  (params (AxisValue :type Float%20%28single-precision%29))
  ;[1 1 1] axis and actions
  (Class|ChaosVehicleMovementComponent|SetThrottleInput (Variables|Default|GetVehicleMovementComponent) AxisValue))

(event Input|MouseEvents|MouseX
  (params (AxisValue :type Float%20%28single-precision%29))
  ;[1 1 1] cam controls
  (Transformation|AddRelativeRotation (Variables|Default|GetSpringArm) (Math|Rotator|MakeRotator 0.0 0.0 AxisValue) false false))

(event Input|MouseEvents|MouseY
  (params (AxisValue :type Float%20%28single-precision%29))
  ;[1 1 1] cam controls
  (Transformation|AddRelativeRotation (Variables|Default|GetSpringArm) (Math|Rotator|MakeRotator 0.0 AxisValue 0.0) false false))

(fn ConstructionScript)