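; BP_MovingRock is an actor that repositions a rock cube relative to the location of a skeletal mesh.
; BeginPlay prints and stores the mesh's start location, though the stored value is not read afterwards.
; While the mesh's world Y lies within a narrow band, Tick snaps the cube to that location with a slight negative Y offset.
; Socket lookups name no socket, and an unfinished looping timer is never run.
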(event Collision|EventActorBeginOverlap
  (params (OtherActor :type Actor%20Object%20Reference)))

(event EventBeginPlay
  (bind _cubeskeletalmesh (Variables|Default|GetCubeSkeletalMesh))
  (bind _returnvalue (Transformation|GetSocketLocation _cubeskeletalmesh "None"))
  (Development|PrintString (Utilities|String|ToString(Vector) _returnvalue))
  (Variables|Default|SetrockStartLoc _returnvalue))

(event EventTick
  (params (DeltaSeconds :type Float%20%28single-precision%29))
  (bind _cubeskeletalmesh (Variables|Default|GetCubeSkeletalMesh))
  (bind _returnvalue (Transformation|GetSocketLocation _cubeskeletalmesh "None"))
  (bind (_x _y _z) (Class|KismetMathLibrary|BreakVector3f _returnvalue))
  (if (and (> _y -1.0) (<= _y 3e+01))
    (Transformation|SetWorldLocation (Variables|Default|GetRockCube) (Math|Vector|MakeVector _x (- _y 0.1) _z) false false)))

(fn ConstructionScript)